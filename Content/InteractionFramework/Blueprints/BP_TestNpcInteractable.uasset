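; BP_TestNpcInteractable is a test NPC for the interaction framework that takes keys from whoever talks to it.
; When talk requirements are met, its current state ID selects the key to take and the next state, progressing from wanting the blue key to the red key to done.
; If the state change succeeds, it removes that key from the interactor's KeyringComponent and prints the lost key.
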(event EventOnTalkRequirementsMet
  (params (Interactor :type Actor%20Object%20Reference))
  (switch name (Variables|Default|GetCurrentStateId)
    (:WantBlueKey
      (Variables|Default|SetInKeyId "BlueKey")
      (Variables|Default|SetInStateId "WantRedKey"))
    (:WantRedKey
      (Variables|Default|SetInKeyId "RedKey")
      (Variables|Default|SetInStateId "Done")))
  (bind _returnvalue (Class|InteractableNpcActorBase|SetNpcState (Variables|Default|GetInStateId)))
  (if _returnvalue
    (bind _returnvalue_2 (Class|KeyringComponent|RemoveKey (Actor|GetComponentbyClass Interactor "/Script/InteractionFramework.KeyringComponent") (Variables|Default|GetInKeyId)))
    (if _returnvalue_2
      (Development|PrintString (Utilities|String|Append "You lost: " (Utilities|String|ToString(Name) (Variables|Default|GetInKeyId)))))))

(fn ConstructionScript)