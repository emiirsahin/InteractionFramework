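; Test interactable for the interaction framework that flips between two hurdle states and consumes a colored key on each interaction.
; When interaction is available, the current state picks the target state and the red or blue key.
; It changes state first, then removes the key from the interactor's KeyringComponent, so a failed removal does not revert the state.
; Focus swaps the cube's material, and outcomes print debug strings.
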(event EventOnFocusEnd
  (params (Interactor :type Actor%20Object%20Reference))
  (Rendering|Material|SetMaterial (Variables|Default|GetCube) 0 "/Engine/BasicShapes/BasicShapeMaterial.BasicShapeMaterial"))

(event EventOnFocusStart
  (params (Interactor :type Actor%20Object%20Reference))
  (Rendering|Material|SetMaterial (Variables|Default|GetCube) 0 "/AnimationSharing/AnimSharingRed.AnimSharingRed"))

(event EventOnInteractUnavailable
  (params (Interactor :type Actor%20Object%20Reference) (MissingMessages :type Array%20of%20Texts))
  (Development|PrintString "Interaction Failed with obj3"))

(event EventOnInteractAvailable
  (params (Interactor :type Actor%20Object%20Reference))
  (switch name (Variables|Default|GetCurrentStateId)
    (:Hurdle1
      (Variables|Default|SetInKeyId "RedKey")
      (Variables|Default|SetInStateId "Hurdle2"))
    (:Hurdle2
      (Variables|Default|SetInKeyId "BlueKey")
      (Variables|Default|SetInStateId "Hurdle1")))
  (bind _returnvalue (Class|InteractableActorBase|SetInteractionState (Variables|Default|GetInStateId)))
  (if _returnvalue
    (bind _returnvalue_2 (Class|KeyringComponent|RemoveKey (Actor|GetComponentbyClass Interactor "/Script/InteractionFramework.KeyringComponent") (Variables|Default|GetInKeyId)))
    (if _returnvalue_2
      (Development|PrintString "Interaction Success with obj3, you lost the key")
      (else
        (Development|PrintString "Couldn't remove key")))
    (else
      (Development|PrintString "Couldn't change state"))))

(fn ConstructionScript)