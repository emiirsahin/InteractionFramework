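; BP_TestInteractable2 is a test interactable for the interaction framework that toggles between two interaction states.
; When interaction is available, it switches on CurrentStateId, requests the other state through SetInteractionStateById and prints whether the change succeeded.
; An unavailable interaction prints a failure message.
; Focus start and end swap the Cube's material between a red highlight and the basic shape material.
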(event EventOnFocusEnd
  (params (Interactor :type Actor%20Object%20Reference))
  (Rendering|Material|SetMaterial (Variables|Default|GetCube) 0 "/Engine/BasicShapes/BasicShapeMaterial.BasicShapeMaterial"))

(event EventOnFocusStart
  (params (Interactor :type Actor%20Object%20Reference))
  (Rendering|Material|SetMaterial (Variables|Default|GetCube) 0 "/AnimationSharing/AnimSharingRed.AnimSharingRed"))

(event EventOnInteractUnavailable
  (params (Interactor :type Actor%20Object%20Reference) (MissingMessages :type Array%20of%20Texts))
  (Development|PrintString "Interaction Failed with obj2"))

(event EventOnInteractAvailable
  (params (Interactor :type Actor%20Object%20Reference))
  (switch name (Variables|Default|GetCurrentStateId)
    (:State1
      (Variables|Default|SetInStateId "State2"))
    (:State2
      (Variables|Default|SetInStateId "State1")))
  (bind _returnvalue (Class|InteractableActorBase|SetInteractionStatebyId (Variables|Default|GetInStateId)))
  (if _returnvalue
    (Development|PrintString "Interaction Success with obj2")
    (else
      (Development|PrintString "Couldn't change state"))))

(fn ConstructionScript)